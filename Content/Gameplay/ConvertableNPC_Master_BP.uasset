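; Master Blueprint for a convertible NPC that is either repented or damned when a ThirdPersonCharacter overlaps it.
; A DoOnce limits conversion to one time and sends a moral value message through MoralInterface after looping its implementers.
; The character's LMBRMB flag selects the Repented animation, followed by delayed destruction, or the Damned animation, with no destruction.
; The SaveCast montage check has empty branches.
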(event `self.ReceiveActorBeginOverlap`
  (params (OtherActor :type "Actor Object Reference"))
  (bind _skeletalmeshcomponent (`self.SkeletalMeshComponent`))
  (bind _asthird_person_character (cast `/Game/ThirdPersonBP/Blueprints/ThirdPersonCharacter` OtherActor))
  (if (`AnimInstance.Montage_IsPlaying` (`SkeletalMeshComponent.GetAnimInstance` (`Character.Mesh` _asthird_person_character)) "/Game/Models/Remy/SaveCast_Montage.SaveCast_Montage")
    _
    (else
      _))
  (`/Engine/EditorBlueprintResources/StandardMacros.DoOnce` false
    (:`Completed`
      (bind _outactors (`GameplayStatics.GetAllActorsWithInterface` "/Game/Gameplay/MoralInterface.MoralInterface_C"))
      (for _array_element _outactors
        _)
      (message `/Game/Gameplay/MoralInterface.SendMoralValue` _array_element)
      (if (`/Game/ThirdPersonBP/Blueprints/ThirdPersonCharacter.LMB/RMB` _asthird_person_character)
        (`SkeletalMeshComponent.PlayAnimation` _skeletalmeshcomponent "/Game/Animations/Repented.Repented" false)
        (`KismetSystemLibrary.Delay` 5.0)
        (`self.K2_DestroyActor`)
        (else
          (`SkeletalMeshComponent.PlayAnimation` _skeletalmeshcomponent "/Game/Animations/Damned.Damned" false))))))

(fn `UserConstructionScript`)